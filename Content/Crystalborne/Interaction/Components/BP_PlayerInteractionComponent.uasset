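; Player interaction component that finds BPI_Interactable actors with a camera-forward line trace and lets the owner interact with them.
; Focus changes send enter/exit messages, toggle an overlay highlight material and refresh the prompt; leaving a target clears it, so a new one registers on a later trace.
; TryInteract checks CanInteract first.
; An externally supplied widget shows text, failure reason and Enhanced Input key, projected above the target.
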(fn `HideInteractionPrompt`
  (`/Engine/EditorBlueprintResources/StandardMacros.IsValid` (`self.InteractionPromptWidget`)
    (:`Is Valid`
      (`Widget.SetVisibility` (`self.InteractionPromptWidget`) "Collapsed"))))

(fn `InitializeInteraction`
  (params (Camera :type "CameraComponent Object Reference"))
  (set `self.InteractionCamera` Camera))

(fn `PerformInteractionTrace`
  (bind _interactioncamera (`self.InteractionCamera`))
  (bind _returnvalue (`SceneComponent.K2_GetComponentLocation` _interactioncamera))
  (bind (_outhit _returnvalue_2) (`KismetSystemLibrary.LineTraceSingle` _returnvalue (+ _returnvalue (* (`SceneComponent.GetForwardVector` _interactioncamera) (`self.InteractionRange`))) "TraceTypeQuery1" false (`|MakeArray` (`self.GetOwner`))))
  (if _returnvalue_2
    (bind (_bblockinghit _binitialoverlap _time _distance _location _impactpoint _normal _impactnormal _physmat _hitactor) (`GameplayStatics.BreakHitResult` _outhit))
    (if (`KismetSystemLibrary.DoesImplementInterface` _hitactor "/Game/Crystalborne/Interaction/Interfaces/BPI_Interactable.BPI_Interactable_C")
      (`self.UpdateInteractionTarget` _hitactor)
      (else
        (`self.UpdateInteractionTarget` null)))
    (else
      (`self.UpdateInteractionTarget` null))))

(fn `RefreshInteractionPrompt`
  (bind _interactionpromptwidget (`self.InteractionPromptWidget`))
  (`/Engine/EditorBlueprintResources/StandardMacros.IsValid` (`self.InteractionPromptWidget`)
    (:`Is Valid`
      (`/Engine/EditorBlueprintResources/StandardMacros.IsValid` (`self.CurrentInteractionTarget`)
        (:`Is Valid`
          (`Widget.SetVisibility` (`self.InteractionPromptWidget`) "Visible")
          (bind _interactiontext (message `/Game/Crystalborne/Interaction/Interfaces/BPI_Interactable.GetInteractionText` (`self.CurrentInteractionTarget`)))
          (`/Game/Crystalborne/UI/HUD/WBP_InteractionPrompt.SetInteractionText` (`self.InteractionPromptWidget`) _interactiontext)
          (bind (_caninteract _failurereason) (message `/Game/Crystalborne/Interaction/Interfaces/BPI_Interactable.CanInteract` (`self.CurrentInteractionTarget`) (`self.GetOwner`)))
          (if _caninteract
            (`/Game/Crystalborne/UI/HUD/WBP_InteractionPrompt.SetFailureReason` _interactionpromptwidget "")
            (else
              (`/Game/Crystalborne/UI/HUD/WBP_InteractionPrompt.SetFailureReason` _interactionpromptwidget _failurereason))))
        (:`Is Not Valid`
          (`self.HideInteractionPrompt`))))))

(fn `SetInteractionHighlight`
  (params (TargetActor :type "Actor Object Reference") (bHighlightEnabled :type Boolean))
  (`/Engine/EditorBlueprintResources/StandardMacros.IsValid` TargetActor
    (:`Is Valid`
      (for _array_element (`Actor.K2_GetComponentsByClass` TargetActor "/Script/Engine.MeshComponent")
        (if bHighlightEnabled
          (`MeshComponent.SetOverlayMaterial` _array_element "/Game/Crystalborne/Art/Materials/M_InteractionHighlight.M_InteractionHighlight" false 0)
          (else
            (`MeshComponent.SetOverlayMaterial` _array_element null false 0)))))))

(fn `SetInteractionPromptWidget`
  (params (Widget :type "/Game/Crystalborne/UI/HUD/WBP_InteractionPrompt Object Reference"))
  (set `self.InteractionPromptWidget` Widget))

(fn `TryInteract`
  (bind _currentinteractiontarget (`self.CurrentInteractionTarget`))
  (`/Engine/EditorBlueprintResources/StandardMacros.IsValid` _currentinteractiontarget
    (:`Is Valid`
      (bind (_caninteract _failurereason) (message `/Game/Crystalborne/Interaction/Interfaces/BPI_Interactable.CanInteract` _currentinteractiontarget (`self.GetOwner`)))
      (if _caninteract
        (message `/Game/Crystalborne/Interaction/Interfaces/BPI_Interactable.Interact` (`self.CurrentInteractionTarget`) (`self.GetOwner`))
        (else
          (`KismetSystemLibrary.PrintString` (`KismetTextLibrary.Conv_TextToString` _failurereason)))))))

(fn `UpdateInteractionKey`
  (bind _returnvalue (`EnhancedInputSubsystemInterface.QueryKeysMappedToAction` (pcsubsystem `EnhancedInputLocalPlayerSubsystem` (`GameplayStatics.GetPlayerController` 0)) "/Game/Crystalborne/Core/Input/Actions/IA_Interact.IA_Interact"))
  (if (> (`KismetArrayLibrary.Array_Length` _returnvalue) 0)
    (`KismetSystemLibrary.PrintString` "key found")
    (`/Game/Crystalborne/UI/HUD/WBP_InteractionPrompt.SetInteractionKey` (`self.InteractionPromptWidget`) (`KismetInputLibrary.Key_GetDisplayName` (`|GetArrayItem` _returnvalue)))
    (else
      (`KismetSystemLibrary.PrintString` "No key found"))))

(fn `UpdateInteractionPromptPosition`
  (bind _interactionpromptwidget (`self.InteractionPromptWidget`))
  (bind (_screenposition _returnvalue) (`WidgetLayoutLibrary.ProjectWorldLocationToWidgetPosition` (`GameplayStatics.GetPlayerController` 0) (+ (`Actor.K2_GetActorLocation` (`self.CurrentInteractionTarget`)) (`self.InteractionPromptWorldOffset`))))
  (`/Engine/EditorBlueprintResources/StandardMacros.IsValid` (`self.InteractionPromptWidget`)
    (:`Is Valid`
      (`/Engine/EditorBlueprintResources/StandardMacros.IsValid` (`self.CurrentInteractionTarget`)
        (:`Is Valid`
          (if _returnvalue
            (`UserWidget.SetAlignmentInViewport` _interactionpromptwidget (0.5 1.0))
            (`UserWidget.SetPositionInViewport` _interactionpromptwidget _screenposition false)))))))

(fn `UpdateInteractionTarget`
  (params (NewTarget :type "Actor Object Reference"))
  (bind _currentinteractiontarget (`self.CurrentInteractionTarget`))
  (if (!= (`self.CurrentInteractionTarget`) NewTarget)
    (`/Engine/EditorBlueprintResources/StandardMacros.IsValid` _currentinteractiontarget
      (:`Is Valid`
        (message `/Game/Crystalborne/Interaction/Interfaces/BPI_Interactable.ExitFocus` _currentinteractiontarget (`self.GetOwner`))
        (`self.SetInteractionHighlight` _currentinteractiontarget)
        (bind _output_get (set `self.CurrentInteractionTarget` null))
        (`/Engine/EditorBlueprintResources/StandardMacros.IsValid` _output_get
          (:`Is Valid`
            (message `/Game/Crystalborne/Interaction/Interfaces/BPI_Interactable.EnterFocus` _output_get (`self.GetOwner`))
            (`self.SetInteractionHighlight` _output_get true)
            (`self.RefreshInteractionPrompt`))
          (:`Is Not Valid`
            (`self.RefreshInteractionPrompt`))))
      (:`Is Not Valid`
        (bind _output_get_2 (set `self.CurrentInteractionTarget` NewTarget))
        (`/Engine/EditorBlueprintResources/StandardMacros.IsValid` _output_get_2
          (:`Is Valid`
            (message `/Game/Crystalborne/Interaction/Interfaces/BPI_Interactable.EnterFocus` _output_get_2 (`self.GetOwner`))
            (`self.SetInteractionHighlight` _output_get_2 true)
            (`self.RefreshInteractionPrompt`))
          (:`Is Not Valid`
            (`self.RefreshInteractionPrompt`)))))))