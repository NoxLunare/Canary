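; BP_TestInteractable is a test actor for exercising the interaction system.
; Focus enter, focus exit and interact events each print a debug string to confirm they fired.
; CanInteract always returns false with an "Interaction is currently unavailable" reason, so it represents a blocked interactable.
; It also supplies fixed prompt text and a fixed interaction type.
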(event `/Game/Crystalborne/Interaction/Interfaces/BPI_Interactable.EnterFocus`
  (params (Interactor :type "Actor Object Reference"))
  (`KismetSystemLibrary.PrintString` "ENTER FOCUS"))

(event `/Game/Crystalborne/Interaction/Interfaces/BPI_Interactable.ExitFocus`
  (params (Interactor :type "Actor Object Reference"))
  (`KismetSystemLibrary.PrintString` "EXIT FOCUS"))

(event `/Game/Crystalborne/Interaction/Interfaces/BPI_Interactable.Interact`
  (params (Interactor :type "Actor Object Reference"))
  (`KismetSystemLibrary.PrintString` "INTERACTION SUCCESSFUL"))

(fn `CanInteract`
  (params (Interactor :type "Actor Object Reference"))
  (returns (CanInteract :type Boolean) (FailureReason :type Text))
  (return false "Interaction is currently unavailable"))

(fn `GetInteractionText`
  (returns (InteractionText :type Text))
  (return "Interact with object"))

(fn `GetInteractionType`
  (returns (InteractionType :type "/Game/Crystalborne/Data/Enums/E_InteractionType Enum"))
  (return "NewEnumerator0"))

(fn `UserConstructionScript`)